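; BP_SlopeTracer solves a two-part Day 3 puzzle, counting trees hit along slopes through a horizontally wrapping grid.
; Data table rows become an IntVector-keyed map, spawned as TheField instanced meshes with tree state in custom data.
; CountHitTrees steps across the map, flagging hit instances through a second custom data value.
; Test and run events show Part01's single-slope count or Part02's Int64 product across TestSlopes on a TextRender.
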(event Custom|RunPart02
  (bind _localhittreesproduct1 (CallFunction|Part02 (Variables|Default|GetData01)))
  (Rendering|Components|TextRender|SetText (Variables|Default|GetTextRender) (Utilities|Text|ToText(String) _localhittreesproduct1)))

(event Custom|TestPart01
  (bind _numhittrees (CallFunction|Part01 (Variables|Default|GetTestData01)))
  (Rendering|Components|TextRender|SetText (Variables|Default|GetTextRender) (Utilities|Text|ToText(Integer) _numhittrees)))

(event Custom|TestPart02
  (bind _localhittreesproduct1 (CallFunction|Part02 (Variables|Default|GetTestData01)))
  (Rendering|Components|TextRender|SetText (Variables|Default|GetTextRender) (Utilities|Text|ToText(String) _localhittreesproduct1)))

(event Custom|RunPart01
  (bind _numhittrees (CallFunction|Part01 (Variables|Default|GetData01)))
  (Rendering|Components|TextRender|SetText (Variables|Default|GetTextRender) (Utilities|Text|ToText(Integer) _numhittrees)))

(fn ConstructionScript)

(fn ConvertinDatatoGridData
  (params (InData :type Data%20Table%20Object%20Reference))
  (bind (_xsize _ysize) (CallFunction|GetDataDimensions InData))
  (LocalVariables|SetXSize _xsize)
  (LocalVariables|SetYSize _ysize)
  (bind _outrownames (DataTable|GetDataTableRowNames InData))
  (for _array_element _outrownames
    (bind _returnvalue (Utilities|GetDataTableRow InData _array_element)
      (:then
        (for _index (range 0 (LocalVariables|GetXSize))
          (Utilities|Map|Add (LocalVariables|GetLocalOut) (Utilities|Struct|MakeIntVector _index (LocalVariables|GetCurrentY) 0) (Utilities|Struct|MakeDay03TreeData (Utilities|Array|Get(acopy) (Utilities|Struct|BreakDay03Struct _returnvalue) _index) 0)))
        (Math|Integer|IncrementInt (LocalVariables|GetCurrentY)))))
  (return (LocalVariables|GetLocalOut)))

(fn GetDataDimensions
  (params (Table :type Data%20Table%20Object%20Reference))
  (bind _outrownames (DataTable|GetDataTableRowNames Table))
  (bind _returnvalue (Utilities|GetDataTableRow Table (Utilities|Array|Get(acopy) _outrownames))
    (:then
      (return (Utilities|Array|Length (Utilities|Struct|BreakDay03Struct _returnvalue)) (Utilities|Array|Length _outrownames)))))

(fn PopulateISM
  (params (GridData :type Map%20of%20Int%20Vector%20Structures%20to%20Structs))
  (bind _thefield (Variables|Default|GetTheField))
  (bind _staticmesh (Variables|/Script/Engine.StaticMeshComponent|GetStaticMesh _thefield))
  (bind _returnvalue (StaticMesh|GetBounds _staticmesh))
  (bind _boxextent (Math|BoxSphereBounds|BreakBoxSphereBounds _returnvalue))
  (bind (_x _y) (Math|Vector|BreakVector _boxextent))
  (Components|InstancedStaticMesh|ClearInstances _thefield)
  (LocalVariables|SetXIncrement _x)
  (LocalVariables|SetYIncrement _y)
  (bind _keys (Utilities|Map|Keys GridData))
  (for _array_element _keys
    (bind _returnvalue_2 (Components|InstancedStaticMesh|AddInstance (Variables|Default|GetTheField) (Math|Transform|MakeTransform (Math|Vector|MakeVector (* (.X (Utilities|Struct|BreakIntVector _array_element)) (LocalVariables|GetXIncrement)) (* (.Y (Utilities|Struct|BreakIntVector _array_element)) (LocalVariables|GetYIncrement)) 0.0))))
    (Components|InstancedStaticMesh|SetCustomDataValue (Variables|Default|GetTheField) _returnvalue_2 0 (Math|Conversions|ToFloat(Boolean) (.IsTree (Utilities|Struct|BreakDay03TreeData (.Value (Utilities|Map|Find GridData _array_element))))) false)
    (bind _structout (Utilities|Struct|SetmembersinDay03TreeData (.Value (Utilities|Map|Find GridData _array_element)) _returnvalue_2))
    (Utilities|Map|Add (LocalVariables|GetInstancedData) _array_element _structout))
  (return (LocalVariables|GetInstancedData)))

(fn Part01
  (params (InData :type Data%20Table%20Object%20Reference))
  (bind (_xsize _ysize) (CallFunction|GetDataDimensions InData))
  (bind _outdata (CallFunction|ConvertinDatatoGridData InData))
  (bind _output_get (LocalVariables|SetGridData _outdata))
  ;[1 1 1] TODO: Something in here isn't working to get instance IDs set and passed out
  (bind _outdata_2 (CallFunction|PopulateISM _output_get))
  (bind _hittrees (CallFunction|CountHitTrees (Variables|Default|GetRise) (Variables|Default|GetRun) _xsize _ysize _outdata_2))
  (return _hittrees))

(fn CountHitTrees
  (params (Run :type Integer%20%28by%20ref%29) (Rise :type Integer%20%28by%20ref%29) (Width :type Integer%20%28by%20ref%29) (Height :type Integer%20%28by%20ref%29) (InGrid :type Map%20of%20Int%20Vector%20Structures%20to%20Structs))
  (for _index (range 0 Height)
    (bind _output_get (LocalVariables|SetPointer (Utilities|Struct|MakeIntVector (Math|Integer|%(Integer) (+ (.X (Utilities|Struct|BreakIntVector (LocalVariables|GetPointer))) Run) Width) (+ (.Y (Utilities|Struct|BreakIntVector (LocalVariables|GetPointer))) Rise))))
    (if (.ReturnValue (Utilities|Map|Find InGrid _output_get))
      (if (.IsTree (Utilities|Struct|BreakDay03TreeData (.Value (Utilities|Map|Find InGrid _output_get))))
        (Math|Integer|IncrementInt (LocalVariables|GetLocalHitTrees)
          (:%20%20
            (Components|InstancedStaticMesh|SetCustomDataValue (Variables|Default|GetTheField) (.InstanceID (Utilities|Struct|BreakDay03TreeData (.Value (Utilities|Map|Find InGrid _output_get)))) 1 1.0 false))))
      (else
        (Development|PrintString (Utilities|String|Append "Attempted to access out of bounds int vector" " " (Utilities|String|ToString(Integer) _output_get))))))
  (return (LocalVariables|GetLocalHitTrees)))

(fn Part02
  (params (InData :type Data%20Table%20Object%20Reference))
  (bind (_xsize _ysize) (CallFunction|GetDataDimensions InData))
  (bind _outdata (CallFunction|ConvertinDatatoGridData InData))
  (LocalVariables|SetXSize _xsize)
  (LocalVariables|SetYSize _ysize)
  (bind _outdata_2 (CallFunction|PopulateISM _outdata))
  (LocalVariables|SetGridData _outdata_2)
  (for _array_element (Variables|Default|GetTestSlopes)
    (bind _hittrees (CallFunction|CountHitTrees (.X (Utilities|Struct|BreakIntVector _array_element)) (.Y (Utilities|Struct|BreakIntVector _array_element)) (LocalVariables|GetXSize) (LocalVariables|GetYSize) (LocalVariables|GetGridData)))
    (LocalVariables|SetLocalHitTreesProduct (* (LocalVariables|GetLocalHitTreesProduct) (Class|KismetMathLibrary|ToInt64(Integer) _hittrees))))
  (return (LocalVariables|GetLocalHitTreesProduct)))