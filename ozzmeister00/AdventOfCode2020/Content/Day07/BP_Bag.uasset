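; BP_Bag is an actor representing one bag, built in the construction script from the BagDataTable row matching its Name.
; The row's color drives a dynamic material instance on the Cube, with zero alpha serving as a flag for a shiny gold look via metallic and roughness parameters.
; Adding child bags is still a TODO with a placeholder print, and a missing row prints an error.
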(event EventBeginPlay)

(event Collision|EventActorBeginOverlap
  (params (OtherActor :type Actor%20Object%20Reference)))

(event EventTick
  (params (DeltaSeconds :type Float%20%28single-precision%29)))

(fn ConstructionScript
  (bind _returnvalue (Utilities|GetDataTableRow (Variables|Default|GetBagDataTable) (Variables|Default|GetName))
    (:then
      (Utilities|FlowControl|Sequence
        (:then_0
          (Variables|Default|SetBagData _returnvalue)
          ;[1 1 1] Set up the material for our bag
          (bind _returnvalue_2 (Rendering|Material|CreateDynamicMaterialInstance (Rendering|Material|GetMaterial (Variables|Default|GetCube) 0) "None" "None" :!class /Script/Engine.KismetMaterialLibrary))
          (bind _output_get (Variables|Default|SetMID _returnvalue_2))
          (Rendering|Material|SetMaterial (Variables|Default|GetCube) 0 _output_get)
          (Rendering|Material|SetVectorParameterValue (Variables|Default|GetMID) "Color" (Math|Conversions|ToLinearColor(Color) (.Color (Utilities|Struct|BreakDay07Struct (Variables|Default|GetBagData)))) :!class /Script/Engine.MaterialInstanceDynamic)
          (if (== (.A (Math|Color|BreakColor (.Color (Utilities|Struct|BreakDay07Struct (Variables|Default|GetBagData))))) 0)
            (Rendering|Material|SetScalarParameterValue (Variables|Default|GetMID) "Roughness" 0.0 :!class /Script/Engine.MaterialInstanceDynamic)
            (Rendering|Material|SetScalarParameterValue (Variables|Default|GetMID) "Metallic" 1.0 :!class /Script/Engine.MaterialInstanceDynamic)))
        (:then_1
          ;[1 1 1] Todo add this bag's children
          (Development|PrintString "Hello"))))
    (:RowNotFound
      (Development|PrintString (Utilities|String|Append "Failed to find row with name " (Utilities|String|ToString(Name) (Variables|Default|GetName)))))))