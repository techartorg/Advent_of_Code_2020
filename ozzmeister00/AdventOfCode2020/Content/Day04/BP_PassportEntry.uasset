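; BP_PassportEntry holds one Day 4 passport record, copied from a struct by Populate, and validates it.
; IsValidCIDOptional checks that every field except CountryID is present, treating -1 or empty strings as missing.
; IsValidData applies field rules: year ranges, unit-aware height limits, allowed eye codes, nine-character passport IDs, and six-character hex hair colors checked through HairColorIsValid.
; ToString concatenates all fields into one string.
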(event Custom|Populate
  (bind _struct (Variables|Default|GetStruct))
  (bind (_birthyear _issueyear _expirationyear _height _haircolor _eyecolor _passportid _countryid) (Utilities|Struct|BreakDay04Struct _struct))
  (Variables|Default|SetBirthYear _birthyear)
  (Variables|Default|SetIssueYear _issueyear)
  (Variables|Default|SetExpirationYear _expirationyear)
  (Variables|Default|SetHeight _height)
  (Variables|Default|SetHairColor _haircolor)
  (Variables|Default|SetEyeColor _eyecolor)
  (Variables|Default|SetPassportID _passportid)
  (Variables|Default|SetCountryID _countryid))

(fn IsValidCIDOptional
  (return (Math|Boolean|ANDBoolean (> (Variables|Default|GetBirthYear) -1) (> (Variables|Default|GetIssueYear) -1) (> (Variables|Default|GetExpirationYear) -1) (not (Utilities|Array|IsEmpty (Variables|Default|GetHeight))) (not (Utilities|Array|IsEmpty (Variables|Default|GetHairColor))) (not (Utilities|Array|IsEmpty (Variables|Default|GetEyeColor))) (not (Utilities|Array|IsEmpty (Variables|Default|GetPassportID))))))

(fn ToString
  (return (Utilities|String|Append (Utilities|String|ToString(Integer) (Variables|Default|GetBirthYear)) " " (Utilities|String|ToString(Integer) (Variables|Default|GetIssueYear)) " " (Utilities|String|ToString(Integer) (Variables|Default|GetExpirationYear)) " " (Variables|Default|GetHeight) " " (Variables|Default|GetHairColor) " " (Variables|Default|GetEyeColor) " " (Variables|Default|GetPassportID) " " (Utilities|String|ToString(Integer) (Variables|Default|GetCountryID)))))

(fn IsValidData
  (bind _birthyear (Variables|Default|GetBirthYear))
  (bind _issueyear (Variables|Default|GetIssueYear))
  (bind _expirationyear (Variables|Default|GetExpirationYear))
  (bind _passportid (Variables|Default|GetPassportID))
  (return (Math|Boolean|ANDBoolean (and (> _birthyear 1919) (< _birthyear 2003)) (and (>= _issueyear 2010) (<= _issueyear 2020)) (and (>= _expirationyear 2020) (<= _expirationyear 2030)) (CallFunction|ValidateHeight (Variables|Default|GetHeight)) (CallFunction|ValidateHairColor (Variables|Default|GetHairColor)) (Utilities|Array|ContainsItem (Utilities|Array|MakeArray "amb" "blu" "brn" "gry" "grn" "hzl" "oth") (Variables|Default|GetEyeColor)) (and (== (Utilities|String|Len _passportid) 9) (> (Math|Conversions|ToInteger(Byte) _passportid) 0)))))

(fn ValidateHeight
  (params (Height :type String%20%28by%20ref%29))
  (bind _lefts (Utilities|String|Split Height "in"))
  (bind _lefts_2 (Utilities|String|Split Height "cm"))
  (bind _returnvalue (Math|Conversions|ToInteger(Byte) _lefts_2))
  (bind _returnvalue_2 (Math|Conversions|ToInteger(Byte) _lefts))
  (if (Utilities|String|Contains Height "cm")
    (return (and (>= _returnvalue 150) (<= _returnvalue 193)))
    (elif (Utilities|String|Contains Height "in")
      (return (and (>= _returnvalue_2 59) (<= _returnvalue_2 76)))
      (else
        (return false)))))

(fn ValidateHairColor
  (params (HairColor :type String%20%28by%20ref%29))
  (bind (_lefts _rights _returnvalue) (Utilities|String|Split HairColor "#"))
  (bind _returnvalue_2 (Utilities|String|Len _rights))
  (bind _returnvalue_3 (== _returnvalue_2 6))
  (if _returnvalue
    (if _returnvalue_3
      (bind _returnvalue_4 (Class|PassportEntry|HairColorIsValid (Utilities|String|Append "#" _rights)))
      (return _returnvalue_4)
      (else
        (return _returnvalue_3)))
    (else
      (return false))))