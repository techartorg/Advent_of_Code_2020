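; Day 7 puzzle solver that overrides Part01 and Part02 to answer shiny gold bag nesting questions from a DataTable of bag rules.
; Part01 recursively climbs each row's Parents, gathering bag names into a hierarchy, then counts them excluding shiny gold.
; Part02 recurses down through Contents, repeating per contained quantity to count every nested bag one by one, minus the starting bag.
; Both recursive helpers print each bag they visit.
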(event EventBeginPlay)

(event Collision|EventActorBeginOverlap
  (params (OtherActor :type Actor%20Object%20Reference)))

(event EventTick
  (params (DeltaSeconds :type Float%20%28single-precision%29)))

(fn ConstructionScript
  (|CallParentFunction))

(fn Part01
  (params (InData :type Data%20Table%20Object%20Reference))
  (|CallParentFunction InData)
  (bind _hierarchycount (CallFunction|ParseBagTreeUp InData (Variables|Default|GetShinyGold) (LocalVariables|GetHierarchy)))
  (Utilities|Set|Remove _hierarchycount (Variables|Default|GetShinyGold))
  (return (Utilities|Set|Length _hierarchycount)))

(fn ParseBagTreeDown
  (params (DataTable :type Data%20Table%20Object%20Reference) (BagID :type Name%20%28by%20ref%29) (BagCount :type Integer%20%28by%20ref%29))
  (Development|PrintString (Utilities|String|ToString(Name) BagID))
  (Math|Integer|IncrementInt BagCount
    (:%20%20
      (bind _returnvalue (Utilities|GetDataTableRow DataTable BagID)
        (:then
          (bind _keys (Utilities|Map|Keys (.Contents (Utilities|Struct|BreakDay07Struct _returnvalue))))
          (for _array_element _keys
            (for _index (range 1 (.Value (Utilities|Map|Find (.Contents (Utilities|Struct|BreakDay07Struct _returnvalue)) _array_element)))
              (CallFunction|ParseBagTreeDown DataTable _array_element BagCount)))
          (return))))))

(fn ParseBagTreeUp
  (params (InData :type Data%20Table%20Object%20Reference) (BagName :type Name) (InHierarchy :type Set%20of%20Names))
  (Development|PrintString (Utilities|String|ToString(Name) BagName))
  (Utilities|Set|Add InHierarchy BagName)
  (bind _returnvalue (Utilities|GetDataTableRow InData BagName)
    (:then
      (for _array_element (Utilities|Struct|BreakDay07Struct _returnvalue)
        (CallFunction|ParseBagTreeUp InData _array_element InHierarchy))
      (return InHierarchy))))

(fn Part02
  (params (InData :type Data%20Table%20Object%20Reference))
  (|CallParentFunction InData)
  (CallFunction|ParseBagTreeDown InData (Variables|Default|GetShinyGold) (LocalVariables|GetBagCount))
  (return (- (LocalVariables|GetBagCount) 1)))