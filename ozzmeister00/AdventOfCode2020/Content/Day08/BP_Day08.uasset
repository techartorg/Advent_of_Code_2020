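; Day 8 puzzle solver Blueprint that emulates a small accumulate, jump and no-op computer on a program read from a Data Table.
; DataTableToDict builds an index-to-instruction map, which RunProgram executes until an instruction repeats or the pointer passes the end.
; Part01 returns the accumulator from that run.
; Part02 brute-forces swapping one non-zero Jump or NoOperation at a time until no loop occurs, then returns the accumulator.
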(fn ConstructionScript
  (|CallParentFunction))

(fn GetCommand
  (params (Index :type Integer))
  (return (.Value (Utilities|Map|Find (Variables|Default|GetWorkingProgram) Index))))

(fn InitializeComputer
  (params (InProgram :type Map%20of%20Integers%20to%20Structs))
  (Variables|Default|SetWorkingProgram InProgram)
  (Variables|Default|SetCurrentValue 0)
  (Variables|Default|SetCurrentPointer 0)
  (Variables|Default|SetGlobalAccumulate 0)
  (Variables|Default|SetCurrentOperator "NewEnumerator0")
  (Utilities|Set|Clear (Variables|Default|GetVisitedCommands)))

(fn Part01
  (params (InData :type Data%20Table%20Object%20Reference))
  (|CallParentFunction InData)
  (bind _accumulatorvalue (CallFunction|RunProgram (CallFunction|DataTabletoDict InData)))
  (return _accumulatorvalue))

(fn DetectLoop
  (return (Utilities|Set|Contains (Variables|Default|GetVisitedCommands) (Variables|Default|GetCurrentPointer))))

(fn Part02
  (params (InData :type Data%20Table%20Object%20Reference))
  (bind _workingprogram (CallFunction|DataTabletoDict InData))
  (bind _returnvalue (Utilities|Map|Length _workingprogram))
  (Development|PrintString (Utilities|String|ToString(Integer) _returnvalue))
  (bind _index (Utilities|FlowControl|ForLoopwithBreak 0 _returnvalue :!label _label)
    (:LoopBody
      (if (and (or (Utilities|Enum|Equal(Enum) (.Operator (Utilities|Struct|BreakDay08Struct (.Value (Utilities|Map|Find _workingprogram _index)))) "NewEnumerator1") (Utilities|Enum|Equal(Enum) (.Operator (Utilities|Struct|BreakDay08Struct (.Value (Utilities|Map|Find _workingprogram _index)))) "NewEnumerator2")) (!= (.Value (Utilities|Struct|BreakDay08Struct (.Value (Utilities|Map|Find _workingprogram _index)))) 0))
        (bind _output_get (LocalVariables|SetWorkingProgramSwapped (CallFunction|DataTabletoDict InData)))
        (Utilities|Map|Add _output_get _index (Utilities|Struct|MakeDay08Struct (Utilities|Select :Index (.Operator (Utilities|Struct|BreakDay08Struct (.Value (Utilities|Map|Find _workingprogram _index)))) :NewEnumerator0 "NewEnumerator0" :NewEnumerator1 "NewEnumerator2" :NewEnumerator2 "NewEnumerator1") (.Value (Utilities|Struct|BreakDay08Struct (.Value (Utilities|Map|Find _workingprogram _index))))))
        (bind _loopdetected (CallFunction|RunProgram (LocalVariables|GetWorkingProgramSwapped)))
        (Development|PrintString (Utilities|String|ToString(Boolean) _loopdetected))
        (if (not _loopdetected)
          (goto _label Break))))
    (:Completed
      (return (Variables|Default|GetGlobalAccumulate)))))

(fn RunProgram
  (params (InProgram :type Map%20of%20Integers%20to%20Structs))
  (CallFunction|InitializeComputer InProgram)
  (while (and (not (CallFunction|DetectLoop)) (not (CallFunction|PointerOutsideProgram)))
    (Utilities|Set|Add (Variables|Default|GetVisitedCommands) (Variables|Default|GetCurrentPointer))
    (bind _command (CallFunction|GetCommand (Variables|Default|GetCurrentPointer)))
    (switch Utilities|FlowControl|Switch|SwitchonE_Operators (.Operator (Utilities|Struct|BreakDay08Struct _command))
      (:NewEnumerator0
        (Variables|Default|SetGlobalAccumulate (+ (.Value (Utilities|Struct|BreakDay08Struct _command)) (Variables|Default|GetGlobalAccumulate)))
        (Math|Integer|IncrementInt (Variables|Default|GetCurrentPointer)))
      (:NewEnumerator1
        (Variables|Default|SetCurrentPointer (+ (Variables|Default|GetCurrentPointer) (.Value (Utilities|Struct|BreakDay08Struct _command)))))
      (:NewEnumerator2
        (Math|Integer|IncrementInt (Variables|Default|GetCurrentPointer)))))
  (return (Variables|Default|GetGlobalAccumulate) (CallFunction|DetectLoop)))

(fn PointerOutsideProgram
  (return (>= (Variables|Default|GetCurrentPointer) (Utilities|Map|Length (Variables|Default|GetWorkingProgram)))))

(fn DataTabletoDict
  (params (InProgram :type Data%20Table%20Object%20Reference%20%28by%20ref%29))
  (bind _outrownames (DataTable|GetDataTableRowNames InProgram))
  (for _array_element _outrownames
    (bind _returnvalue (Utilities|GetDataTableRow InProgram _array_element)
      (:then
        (Utilities|Map|Add (LocalVariables|GetLocalProgram) (Math|Conversions|ToInteger(Byte) (Utilities|String|ToString(Name) _array_element)) _returnvalue))))
  (return (LocalVariables|GetLocalProgram)))