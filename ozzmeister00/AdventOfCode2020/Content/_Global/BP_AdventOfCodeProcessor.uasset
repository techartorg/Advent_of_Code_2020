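; Base Blueprint processor for Advent of Code puzzles that shows each answer on a text render component.
; Four events run the Part01 and Part02 functions on either test data or real data and write the integer result as text.
; Both part functions are stubs that return zero.
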(event Custom|RunPart02
  (bind _answer (CallFunction|Part02 (Variables|Default|GetData02)))
  (Rendering|Components|TextRender|SetText (Variables|Default|GetTextRender) (Utilities|Text|ToText(Integer) _answer)))

(event Custom|TestPart01
  (bind _answer (CallFunction|Part01 (Variables|Default|GetTestData01)))
  (Rendering|Components|TextRender|SetText (Variables|Default|GetTextRender) (Utilities|Text|ToText(Integer) _answer)))

(event Custom|TestPart02
  (bind _answer (CallFunction|Part02 (Variables|Default|GetTestData02)))
  (Rendering|Components|TextRender|SetText (Variables|Default|GetTextRender) (Utilities|Text|ToText(Integer) _answer)))

(event Custom|RunPart01
  (bind _answer (CallFunction|Part01 (Variables|Default|GetData01)))
  (Rendering|Components|TextRender|SetText (Variables|Default|GetTextRender) (Utilities|Text|ToText(Integer) _answer)))

(fn ConstructionScript)

(fn Part01
  (params (InData :type Data%20Table%20Object%20Reference))
  (return 0))

(fn Part02
  (params (InData :type Data%20Table%20Object%20Reference))
  (return 0))