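; BP_PasswordValidator solves a two-part password puzzle, counting valid DataTable rows and showing the total on a TextRender.
; Separate events run each part on test or real data, looping over every row with that part's rule.
; Part one checks that a letter's occurrence count, found by recursively splitting the string, lies within Min and Max.
; Part two requires the letter at exactly one of those two 1-based positions, using XOR.
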(event Custom|RunPart02
  (CallFunction|Part02 (Variables|Default|GetData01)))

(event Custom|TestPart01
  (CallFunction|Part01 (Variables|Default|GetTestData01)))

(event Custom|TestPart02
  (CallFunction|Part02 (Variables|Default|GetTestData01)))

(event Custom|RunPart01
  (CallFunction|Part01 (Variables|Default|GetData01)))

(event Custom|Part01
  (params (InData :type Data%20Table%20Object%20Reference))
  ;[1 1 1] Iterate over the input test data, and using the Part01 validation function, determine the number of valid passwords in the dataset
  (Variables|Default|SetValidPasswordCount 0) ; Reset our internal counter
  (bind _outrownames (DataTable|GetDataTableRowNames InData)) ; Iterate over all of the rows we got from the input data table
  (for _array_element _outrownames
    (bind _returnvalue (Utilities|GetDataTableRow InData _array_element)
      (:then
        (bind _isvalid (CallFunction|IsPasswordValidPart01 _returnvalue))
        (if _isvalid
          (Math|Integer|IncrementInt (Variables|Default|GetValidPasswordCount))))
      (:RowNotFound
        (Development|PrintString "InvalidRow"))))
  (Rendering|Components|TextRender|SetText (Variables|Default|GetTextRender) (Utilities|Text|ToText(Integer) (Variables|Default|GetValidPasswordCount))))

(event Custom|Part02
  (params (InData :type Data%20Table%20Object%20Reference))
  ;[1 1 1] Run the same iteration loop over our data table as part 01, instead using the part 02 validation function
  (Variables|Default|SetValidPasswordCount 0) ; Reset our internal counter
  (bind _outrownames (DataTable|GetDataTableRowNames InData)) ; Iterate over all of the rows we got from the input data table
  (for _array_element _outrownames
    (bind _returnvalue (Utilities|GetDataTableRow InData _array_element)
      (:then
        (bind _isvalid (CallFunction|IsPasswordValidPart02 _returnvalue))
        (if _isvalid
          (Math|Integer|IncrementInt (Variables|Default|GetValidPasswordCount))))
      (:RowNotFound
        (Development|PrintString "InvalidRow"))))
  (Rendering|Components|TextRender|SetText (Variables|Default|GetTextRender) (Utilities|Text|ToText(Integer) (Variables|Default|GetValidPasswordCount))))

(fn ConstructionScript)

(fn IsPasswordValidPart01
  (params (InParams :type Day%2002%20Struct%20Structure))
  (bind (_min _max _letter _password) (Utilities|Struct|BreakDay02Struct InParams))
  (bind _outcount (CallFunction|RecursiveSplit _password _letter (LocalVariables|GetCount))) ; Recursively split the input password from the left and count how many times we do that to get the number of times a given letter is in the password
  (return (CallFunction|IsBetween _min _max _outcount)))

(fn RecursiveSplit
  (params (InString :type String) (Letter :type String) (InCount :type Integer%20%28by%20ref%29))
  (bind (_lefts _rights _returnvalue) (Utilities|String|Split InString Letter))
  (bind _output_get (LocalVariables|SetCount InCount))
  (if _returnvalue
    (bind _result (Math|Integer|IncrementInt _output_get)
      (:%20%20
        (bind _outcount (CallFunction|RecursiveSplit _rights Letter _result))
        (return _outcount)))
    (else
      (return (LocalVariables|GetCount)))))

(fn IsBetween
  (params (A :type Integer) (B :type Integer) (V :type Integer))
  (return (and (<= A V) (<= V B))))

(fn IsPasswordValidPart02
  (params (InParams :type Day%2002%20Struct%20Structure))
  (bind (_min _max _letter _password) (Utilities|Struct|BreakDay02Struct InParams))
  (bind _returnvalue (Utilities|String|GetCharacterArrayfromString _password))
  (return (Class|KismetMathLibrary|XORBoolean (Utilities|Enum|Equal(Enum) (Utilities|Array|Get(acopy) _returnvalue (- _min 1)) _letter) (Utilities|Enum|Equal(Enum) (Utilities|Array|Get(acopy) _returnvalue (- _max 1)) _letter))))