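; BP_Day05 solves a two-part seat-ID puzzle from binary space partition data tables, displaying test or real results on a TextRender.
; ParseTableToSeatCoords decodes each row's bit fields into column and row coordinates, which both parts convert to seat IDs.
; Part01 returns the highest ID; Part02 sorts the IDs and returns the first gap.
; Despite its name, QuickSortInteger is a selection sort that repeatedly extracts the maximum, then reverses.
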(event Custom|RunPart02
  (bind _myseatid (CallFunction|Part02 (Variables|Default|GetData01)))
  (Rendering|Components|TextRender|SetText (Variables|Default|GetTextRender) (Utilities|Text|ToText(Integer) _myseatid)))

(event Custom|TestPart01
  (bind _seatid (CallFunction|Part01 (Variables|Default|GetTestData01)))
  (Rendering|Components|TextRender|SetText (Variables|Default|GetTextRender) (Utilities|Text|ToText(Integer) _seatid)))

(event Custom|TestPart02
  (bind _myseatid (CallFunction|Part02 (Variables|Default|GetTestData01)))
  (Rendering|Components|TextRender|SetText (Variables|Default|GetTextRender) (Utilities|Text|ToText(Integer) _myseatid)))

(event Custom|RunPart01
  (bind _seatid (CallFunction|Part01 (Variables|Default|GetData01)))
  (Rendering|Components|TextRender|SetText (Variables|Default|GetTextRender) (Utilities|Text|ToText(Integer) _seatid)))

(fn ConstructionScript)

(fn Part01
  (params (InData :type Data%20Table%20Object%20Reference))
  (bind _outseatcoords (CallFunction|ParseTabletoSeatCoords InData))
  (for _array_element _outseatcoords
    (Utilities|Array|Add (LocalVariables|GetSeatIDs) (+ (.X (Utilities|Struct|BreakIntPoint _array_element)) (* (.Y (Utilities|Struct|BreakIntPoint _array_element)) 8))))
  (return (.MaxValue (Math|Integer|MaxOfIntArray (LocalVariables|GetSeatIDs)))))

(fn Part02
  (params (InData :type Data%20Table%20Object%20Reference))
  (for _index (range 0 (* 128 8))
    (Utilities|Set|Add (LocalVariables|GetAllSeatIDs) _index))
  (bind _outseatcoords (CallFunction|ParseTabletoSeatCoords InData))
  (for _array_element _outseatcoords
    (Utilities|Set|Add (LocalVariables|GetSeatIDs) (+ (.X (Utilities|Struct|BreakIntPoint _array_element)) (* (.Y (Utilities|Struct|BreakIntPoint _array_element)) 8))))
  (bind _result (Utilities|Set|ToArray (LocalVariables|GetSeatIDs)))
  (bind _sorted (CallFunction|QuickSortInteger _result))
  (bind (_array_element_2 _array_index) (Utilities|Array|ForEachLoopwithBreak _sorted :!label _label)
    (:LoopBody
      (if (not (== (+ _array_element_2 1) (Utilities|Array|Get(acopy) _sorted (+ _array_index 1)))) ; Since a set is ordered, look to see if the item next in the list is equal to this item + 1, if not, we found our missing seat and can bail out
        (LocalVariables|SetMissingSeat (+ _array_element_2 1))
        (goto _label Break)))
    (:Completed
      (return (LocalVariables|GetMissingSeat)))))

(fn ParseBSPtoXY
  (params (InBSP :type Day%2005%20Struct%20Structure%20%28by%20ref%29))
  (bind (_r64 _r32 _r16 _r8 _r4 _r2 _r1 _s4 _s2 _s1) (Utilities|Struct|BreakDay05Struct InBSP))
  (return (Utilities|Struct|MakeIntPoint (+ (* (Math|Conversions|ToInteger(Boolean) _s4) 4) (* (Math|Conversions|ToInteger(Boolean) _s2) 2) (* (Math|Conversions|ToInteger(Boolean) _s1) 1)) (+ (* (Math|Conversions|ToInteger(Boolean) _r64) 64) (* (Math|Conversions|ToInteger(Boolean) _r32) 32) (* (Math|Conversions|ToInteger(Boolean) _r16) 16) (* (Math|Conversions|ToInteger(Boolean) _r8) 8) (* (Math|Conversions|ToInteger(Boolean) _r4) 4) (* (Math|Conversions|ToInteger(Boolean) _r2) 2) (* (Math|Conversions|ToInteger(Boolean) _r1) 1)))))

(fn ParseTabletoSeatCoords
  (params (Table :type Data%20Table%20Object%20Reference%20%28by%20ref%29))
  (bind _outrownames (DataTable|GetDataTableRowNames Table))
  (for _array_element _outrownames
    (bind _returnvalue (Utilities|GetDataTableRow Table _array_element)
      (:then
        (bind _coords (CallFunction|ParseBSPtoXY _returnvalue))
        (Utilities|Array|Add (LocalVariables|GetLocalSeatIDs) _coords))))
  (return (LocalVariables|GetLocalSeatIDs)))

(fn QuickSortInteger
  (params (Array :type Array%20of%20Integers))
  (bind (_indexofmaxvalue _maxvalue) (Math|Integer|MaxOfIntArray Array))
  (while (> (Utilities|Array|Length Array) 0)
    (Utilities|Array|Add (LocalVariables|GetOutArray) _maxvalue)
    (Utilities|Array|RemoveIndex Array _indexofmaxvalue))
  (Utilities|Array|Reverse (LocalVariables|GetOutArray))
  (return (LocalVariables|GetOutArray)))