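; BP_Day04 is a Day 4 puzzle-solver actor that counts valid passports from Data Tables and shows the count on a TextRender.
; ParseTableToList turns each row into a populated PassportClass object, which does its own validation.
; Part01 counts entries passing IsValidCIDOptional, printing failing indices, while Part02 counts those passing IsValidData.
; Test and Run events pair each part with test or real data; BeginPlay currently calls TestPart02.
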(event Custom|RunPart02
  (bind _validpassports (CallFunction|Part02 (Variables|Default|GetData01)))
  (Rendering|Components|TextRender|SetText (Variables|Default|GetTextRender) (Utilities|Text|ToText(Integer) _validpassports)))

(event Custom|TestPart01
  (bind _validpassports (CallFunction|Part01 (Variables|Default|GetTestData01)))
  (Rendering|Components|TextRender|SetText (Variables|Default|GetTextRender) (Utilities|Text|ToText(Integer) _validpassports)))

(event Custom|TestPart02
  (bind _validpassports (CallFunction|Part02 (Variables|Default|GetTestData02)))
  (Rendering|Components|TextRender|SetText (Variables|Default|GetTextRender) (Utilities|Text|ToText(Integer) _validpassports)))

(event Custom|RunPart01
  (bind _validpassports (CallFunction|Part01 (Variables|Default|GetData01)))
  (Rendering|Components|TextRender|SetText (Variables|Default|GetTextRender) (Utilities|Text|ToText(Integer) _validpassports)))

(event Collision|EventActorBeginOverlap
  (params (OtherActor :type Actor%20Object%20Reference)))

(event EventTick
  (params (DeltaSeconds :type Float%20%28single-precision%29)))

(event EventBeginPlay
  (CallFunction|TestPart02))

(fn ConstructionScript)

(fn Part01
  (params (InData :type Data%20Table%20Object%20Reference))
  (bind _outentries (CallFunction|ParseTabletoList InData))
  (bind _output_get (LocalVariables|SetEntries _outentries))
  (for (_array_element _array_index) _output_get
    (if (Default|IsValidCIDOptional _array_element)
      (Math|Integer|IncrementInt (LocalVariables|GetLocalValidPassports))
      (else
        (Development|PrintString (Utilities|String|ToString(Integer) _array_index)))))
  (return (LocalVariables|GetLocalValidPassports)))

(fn Part02
  (params (InData :type Data%20Table%20Object%20Reference))
  (bind _outentries (CallFunction|ParseTabletoList InData))
  (for _array_element _outentries
    (if (Default|IsValidData _array_element)
      (Math|Integer|IncrementInt (LocalVariables|GetLocalValidPassports))))
  (return (LocalVariables|GetLocalValidPassports)))

(fn ParseTabletoList
  (params (InData :type Data%20Table%20Object%20Reference%20%28by%20ref%29))
  (bind _outrownames (DataTable|GetDataTableRowNames InData))
  (for _array_element _outrownames
    (bind _returnvalue (Utilities|GetDataTableRow InData _array_element)
      (:then
        (bind _returnvalue_2 (Game|ConstructObjectfromClass (Variables|Default|GetPassportClass) self _returnvalue))
        (Default|Populate _returnvalue_2)
        (Utilities|Array|Add (LocalVariables|GetLocalEntries) _returnvalue_2))))
  (return (LocalVariables|GetLocalEntries)))